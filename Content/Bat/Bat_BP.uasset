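; VR bat that motion controllers pick up and drop, with support for a two-handed aiming grip.
; Pickup disables physics and snaps the bat to the holding controller, stored as SecondHand.
; A different controller overlapping FirstHandTrigger becomes FirstHand if BSecondHand is set, though this Blueprint only clears that flag.
; While tracking, Tick takes pitch and yaw from the line between hands and roll from the holding hand.
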(event `/Game/VirtualRealityBP/Blueprints/PickupActorInterface.Pickup`
  (params (AttachTo :type "SceneComponent Object Reference"))
  (if (not (`self.BFirstHandAttached`))
    (`PrimitiveComponent.SetSimulatePhysics` (`self.StaticMeshComponent`) false)
    (`SceneComponent.K2_AttachToComponent` (`self.K2_GetRootComponent`) AttachTo "None" "SnapToTarget" "SnapToTarget" "KeepWorld" false)
    (`SceneComponent.K2_SetRelativeRotation` (`self.StaticMeshComponent`) (`self.OneHandRotation`) false false)
    (set `self.BFirstHandAttached` true)
    (set `self.BSecondHand` false)
    (set `self.BFirstHandTrackingActive` false)
    (set `self.SecondHand` AttachTo)))

(event `/Game/VirtualRealityBP/Blueprints/PickupActorInterface.Drop`
  (`PrimitiveComponent.SetSimulatePhysics` (`self.StaticMeshComponent`) true)
  (`self.K2_DetachFromActor` "KeepWorld" "KeepWorld" "KeepWorld")
  (set `self.BSecondHand` false)
  (set `self.BFirstHandTrackingActive` false))

(event `self.FirstHandTrigger.OnComponentBeginOverlap`
  (params (OverlappedComponent :type "PrimitiveComponent Object Reference") (OtherActor :type "Actor Object Reference") (OtherComp :type "PrimitiveComponent Object Reference") (OtherBodyIndex :type Integer) (bFromSweep :type Boolean) (SweepResult :type "HitResult Structure (by ref)"))
  (if (`self.BSecondHand`)
    (bind _asbp_motion_controller (cast `/Game/VirtualRealityBP/Blueprints/BP_MotionController` OtherActor))
    (bind _motioncontroller (`/Game/VirtualRealityBP/Blueprints/BP_MotionController.MotionController` _asbp_motion_controller))
    (if (!= _motioncontroller (`self.SecondHand`))
      (set `self.BFirstHandTrackingActive` true)
      (set `self.FirstHand` _motioncontroller))))

(event `self.FirstHandTrigger.OnComponentEndOverlap`
  (params (OverlappedComponent :type "PrimitiveComponent Object Reference") (OtherActor :type "Actor Object Reference") (OtherComp :type "PrimitiveComponent Object Reference") (OtherBodyIndex :type Integer))
  (bind (_asbp_motion_controller _bsuccess) (cast `/Game/VirtualRealityBP/Blueprints/BP_MotionController` (`ActorComponent.GetOwner` (`self.FirstHand`)) :!pure true))
  (if (`self.BFirstHandTrackingActive`)
    (`/Engine/EditorBlueprintResources/StandardMacros.IsValid` (`self.FirstHand`)
      (:`Is Valid`
        (if (and _bsuccess (`|EnumInequality` (`/Game/VirtualRealityBP/Blueprints/BP_MotionController.GripState` _asbp_motion_controller) "NewEnumerator2"))
          (set `self.BFirstHandTrackingActive` false :!label _label)
          (set `self.FirstHand` null)
          (`SceneComponent.K2_SetRelativeRotation` (`self.StaticMeshComponent`) (`self.OneHandRotation`) false false)))
      (:`Is Not Valid`
        (goto _label)))))

(event `self.ReceiveTick`
  (params (DeltaSeconds :type "Float (single-precision)"))
  (bind _secondhand (`self.SecondHand`))
  (if (and (`self.BFirstHandTrackingActive`) (`KismetSystemLibrary.IsValid` (`self.FirstHand`)))
    (`SceneComponent.K2_SetWorldRotation` (`self.StaticMeshComponent`) (`KismetMathLibrary.MakeRotator` (.roll (`SceneComponent.K2_GetComponentRotation` _secondhand)) (.pitch (`KismetMathLibrary.FindLookAtRotation` (`SceneComponent.K2_GetComponentLocation` _secondhand) (`SceneComponent.K2_GetComponentLocation` (`self.FirstHand`)))) (.yaw (`KismetMathLibrary.FindLookAtRotation` (`SceneComponent.K2_GetComponentLocation` _secondhand) (`SceneComponent.K2_GetComponentLocation` (`self.FirstHand`))))) false false)))

(fn `UserConstructionScript`)
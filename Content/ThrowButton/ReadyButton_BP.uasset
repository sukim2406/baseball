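; A physical push button that a BP_Bat tip presses to set IsThrowing on the ScoreModeGameInstance.
; When the tip overlaps the collision, a gated Tick makes the button follow the tip's local-space depth, clamped to its press distance.
; Reaching full depth fires the action, and either that or the tip leaving plays a timeline that snaps the button back and then re-enables pressing.
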(event `self.ReceiveTick`
  (params (DeltaSeconds :type "Float (single-precision)"))
  (bind (_buttonstartlocation_x _buttonstartlocation_y _buttonstartlocation_z) (`KismetMathLibrary.BreakVector` (`self.ButtonStartLocation`)))
  (bind _buttonstartlocation (`self.ButtonStartLocation`))
  (bind _z (.z _buttonstartlocation))
  (bind (_relativelocation_x _relativelocation_y _relativelocation_z) (`KismetMathLibrary.BreakVector` (`SceneComponent.RelativeLocation` (`self.Button`))))
  (`/Engine/EditorBlueprintResources/StandardMacros.Gate` true :!label _label
    (:`Exit`
      (`SceneComponent.K2_SetRelativeLocation` (`self.Button`) (`KismetMathLibrary.MakeVector` (.x (+ _buttonstartlocation (`KismetMathLibrary.MakeVector` 0.0 0.0 (.z (- (`KismetMathLibrary.InverseTransformLocation` (`self.GetTransform`) (`SceneComponent.K2_GetComponentLocation` (`self.Tip`))) (`self.ButtonStartLocation`)))))) (.y (+ _buttonstartlocation (`KismetMathLibrary.MakeVector` 0.0 0.0 (.z (- (`KismetMathLibrary.InverseTransformLocation` (`self.GetTransform`) (`SceneComponent.K2_GetComponentLocation` (`self.Tip`))) (`self.ButtonStartLocation`)))))) (`KismetMathLibrary.FClamp` (.z (+ _buttonstartlocation (`KismetMathLibrary.MakeVector` 0.0 0.0 (.z (- (`KismetMathLibrary.InverseTransformLocation` (`self.GetTransform`) (`SceneComponent.K2_GetComponentLocation` (`self.Tip`))) (`self.ButtonStartLocation`)))))) (- _z (`self.PressDistance`)) _z)) false false)
      (if (`KismetMathLibrary.NearlyEqual_FloatFloat` _relativelocation_z (- _buttonstartlocation_z (`self.PressDistance`)))
        (`self.buttonAction`)
        (`self.ResetButton`)))))

(event `self.Collision.OnComponentBeginOverlap`
  (params (OverlappedComponent :type "PrimitiveComponent Object Reference") (OtherActor :type "Actor Object Reference") (OtherComp :type "PrimitiveComponent Object Reference") (OtherBodyIndex :type Integer) (bFromSweep :type Boolean) (SweepResult :type "HitResult Structure (by ref)"))
  (if (not (`self.DisablePress`))
    (bind _asbp_bat (cast `/Game/Bat/BP_Bat` OtherActor))
    (bind _tip (`/Game/Bat/BP_Bat.Tip` _asbp_bat))
    (if (== _tip OtherComp)
      (set `self.DisablePress` true)
      (set `self.Tip` _tip)
      (set `self.ButtonStartLocation` (`SceneComponent.RelativeLocation` (`self.Button`)))
      (goto _label :!via `Open`))))

(event `ResetButton`
  (`|ExecutionSequence` :!label _label_2
    (:`then_0`
      (goto _label :!via `Close`))
    (:`then_1`
      (bind (_direction _driver) (`Timeline|SnapBack` :!via `PlayFromStart`)
        (:`Update`
          (`SceneComponent.K2_SetRelativeLocation` (`self.Button`) (`KismetMathLibrary.MakeVector` (.x (`self.ButtonStartLocation`)) (.y (`self.ButtonStartLocation`)) (`KismetMathLibrary.Lerp` (.z (`SceneComponent.RelativeLocation` (`self.Button`))) (.z (`self.ButtonStartLocation`)) _driver)) false false))
        (:`Finished`
          (set `self.DisablePress` false))))))

(event `self.Collision.OnComponentEndOverlap`
  (params (OverlappedComponent :type "PrimitiveComponent Object Reference") (OtherActor :type "Actor Object Reference") (OtherComp :type "PrimitiveComponent Object Reference") (OtherBodyIndex :type Integer))
  (bind _asbp_bat (cast `/Game/Bat/BP_Bat` OtherActor))
  (if (== (`/Game/Bat/BP_Bat.Tip` _asbp_bat) OtherComp)
    (goto _label_2)))

(fn `buttonAction`
  (bind _asscore_mode_game_instance (cast `/Game/ScoreModeGameInstance` (`GameplayStatics.GetGameInstance`)))
  (set `/Game/ScoreModeGameInstance.isThrowing` true _asscore_mode_game_instance))

(fn `UserConstructionScript`
  (`TextRenderComponent.K2_SetText` (`self.TextRender`) (`self.ButtonText`)))